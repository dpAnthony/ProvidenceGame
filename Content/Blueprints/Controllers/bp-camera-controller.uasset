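; Camera controller that shows the mouse cursor and drives the first bp-camera-pawn found in the level with pan, zoom and click-to-focus.
; Zoom input changes spring arm length and ortho width together, and pan speed scales with arm length within a clamp.
; Clicking an obj-hex under the cursor starts a timeline that glides the pawn onto it and zooms in.
; Pressing movement afterwards eases back to the stored zoom.
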(event Custom|move-to-focus
  (params (focused-actor :type Actor%20Object%20Reference))
  (bind _camera_pawn_reference (Variables|Default|Getcamera-pawn-reference))
  (if (Utilities|IsValid focused-actor)
    (bind _anim_curve (Timeline|Timeline_0 PlayFromStart)
      (:Update
        (Transformation|SetActorLocation (Variables|Default|Getcamera-pawn-reference) (Math|Vector|Lerp(Vector) (Transformation|GetActorLocation (Variables|Default|Getcamera-pawn-reference)) (Transformation|GetActorLocation focused-actor) _anim_curve) false false)
        (Variables|/Script/Engine.SpringArmComponent|SetTargetArmLength (Variables|/Game/Blueprints/Controllers/bp-camera-pawn.bp-camera-pawn_C|GetSpringArm _camera_pawn_reference) (Math|Float|Lerp (Variables|/Script/Engine.SpringArmComponent|GetTargetArmLength (Variables|/Game/Blueprints/Controllers/bp-camera-pawn.bp-camera-pawn_C|GetSpringArm (Variables|Default|Getcamera-pawn-reference))) 7e+02 _anim_curve))
        (Class|CameraComponent|SetOrthoWidth (Variables|/Game/Blueprints/Controllers/bp-camera-pawn.bp-camera-pawn_C|GetCamera _camera_pawn_reference) (Math|Float|Lerp (Variables|/Script/Engine.SpringArmComponent|GetTargetArmLength (Variables|/Game/Blueprints/Controllers/bp-camera-pawn.bp-camera-pawn_C|GetSpringArm (Variables|Default|Getcamera-pawn-reference))) 7e+02 _anim_curve)))
      (:Finished
        (Variables|Default|Setis-zoom-focused true)
        (Variables|/Game/Blueprints/Controllers/bp-camera-pawn.bp-camera-pawn_C|Setfocused-actor (Variables|Default|Getcamera-pawn-reference) 0)))))

(event EventBeginPlay
  (Variables|Default|SetbShowMouseCursor true)
  (bind _outactors (Actor|GetAllActorsOfClass "/Game/Blueprints/Controllers/bp-camera-pawn.bp-camera-pawn_C"))
  (Variables|Default|Setcamera-pawn-reference (Utilities|Array|Get(acopy) _outactors))
  (Variables|Default|Setprevious_zoom 1.5e+03))

(event Input|ActionEvents|InputActionclick
  (params (Key :type Key%20Structure))
  (:Pressed
    (CallFunction|Handle-mouse-click Key))
  (:Released
    (Variables|Default|Setclick-held false)))

(event Input|ActionEvents|InputActionzoom-in
  (params (Key :type Key%20Structure))
  (:Pressed
    (CallFunction|Zoom (* (Variables|Default|Getzoom-speed) -1.0))
    (if (Variables|Default|Getis-zoom-focused)
      (Variables|Default|Setis-zoom-focused false))))

(event Input|ActionEvents|InputActionzoom-out
  (params (Key :type Key%20Structure))
  (:Pressed
    (CallFunction|Zoom (Variables|Default|Getzoom-speed))
    (if (Variables|Default|Getis-zoom-focused)
      (Variables|Default|Setis-zoom-focused false))))

(event Input|ActionEvents|InputActionmovement
  (params (Key :type Key%20Structure))
  (bind _camera_pawn_reference (Variables|Default|Getcamera-pawn-reference))
  (:Pressed
    (if (Variables|Default|Getis-zoom-focused)
      (bind _anim_curve (Timeline|Timeline_1 PlayFromStart)
        (:Update
          (Variables|/Script/Engine.SpringArmComponent|SetTargetArmLength (Variables|/Game/Blueprints/Controllers/bp-camera-pawn.bp-camera-pawn_C|GetSpringArm _camera_pawn_reference) (Math|Float|Lerp (Variables|/Script/Engine.SpringArmComponent|GetTargetArmLength (Variables|/Game/Blueprints/Controllers/bp-camera-pawn.bp-camera-pawn_C|GetSpringArm (Variables|Default|Getcamera-pawn-reference))) (Variables|Default|Getprevious_zoom) _anim_curve))
          (Class|CameraComponent|SetOrthoWidth (Variables|/Game/Blueprints/Controllers/bp-camera-pawn.bp-camera-pawn_C|GetCamera _camera_pawn_reference) (Math|Float|Lerp (Variables|/Script/Engine.SpringArmComponent|GetTargetArmLength (Variables|/Game/Blueprints/Controllers/bp-camera-pawn.bp-camera-pawn_C|GetSpringArm (Variables|Default|Getcamera-pawn-reference))) (Variables|Default|Getprevious_zoom) _anim_curve))
          (Variables|Default|Setis-zoom-focused false))))))

(event Input|AxisEvents|InputAxismove-y
  (params (AxisValue :type Float%20%28single-precision%29))
  (if (not (Audio|Components|Audio|IsPlaying (Variables|Default|GetTimeline_0)))
    (Transformation|SetActorTransform (Variables|Default|Getcamera-pawn-reference) (Utilities|Movement-x (CallFunction|Movement-speed-calc) (Variables|Default|Getfast-move-mult) AxisValue (Variables|Default|Getcamera-pawn-reference)))))

(event Input|AxisEvents|InputAxismove-x
  (params (AxisValue :type Float%20%28single-precision%29))
  (if (not (Audio|Components|Audio|IsPlaying (Variables|Default|GetTimeline_0)))
    (Transformation|SetActorTransform (Variables|Default|Getcamera-pawn-reference) (Utilities|Movement-y AxisValue (CallFunction|Movement-speed-calc) (Variables|Default|Getfast-move-mult) (Variables|Default|Getcamera-pawn-reference)))))

(fn ConstructionScript
  (bind _outactors (Actor|GetAllActorsOfClass "/Game/Blueprints/Controllers/bp-camera-pawn.bp-camera-pawn_C"))
  (Variables|Default|Setcamera-pawn-reference (Utilities|Array|Get(acopy) _outactors))
  (Variables|Default|Settarget-arm-length (Variables|/Script/Engine.SpringArmComponent|GetTargetArmLength (Variables|/Game/Blueprints/Controllers/bp-camera-pawn.bp-camera-pawn_C|GetSpringArm (Variables|Default|Getcamera-pawn-reference)))))

(fn Handle-mouse-click
  (params (key :type Key%20Structure))
  (bind (_bblockinghit _hitactor) (CallFunction|Check-click-hit))
  (if _bblockinghit
    (bind _asobj_hex (Utilities|Casting|CastToobj-hex _hitactor))
    (bind _output_get (Variables|/Game/Blueprints/Controllers/bp-camera-pawn.bp-camera-pawn_C|Setfocused-actor (Variables|Default|Getcamera-pawn-reference) _asobj_hex))
    (CallFunction|Move-to-focus _output_get)))

(fn Check-click-hit
  (bind _returnvalue (Game|GetPlayerController 0))
  (bind _hitresult (Game|Player|GetHitResultUnderCursorbyChannel _returnvalue "TraceTypeQuery1" true))
  (bind (_bblockinghit _binitialoverlap _time _distance _location _impactpoint _normal _impactnormal _physmat _hitactor) (Collision|BreakHitResult _hitresult))
  (return _bblockinghit _hitactor))

(fn Movement-speed-calc
  (return (Math|Float|Clamp(Float) (/ (Variables|/Script/Engine.SpringArmComponent|GetTargetArmLength (Variables|/Game/Blueprints/Controllers/bp-camera-pawn.bp-camera-pawn_C|GetSpringArm (Variables|Default|Getcamera-pawn-reference))) 1e+02) 5.0 2e+01)))

(fn Zoom
  (params (zoom-speed :type Float%20%28single-precision%29))
  (bind _camera_pawn_reference (Variables|Default|Getcamera-pawn-reference))
  (bind _camera (Variables|/Game/Blueprints/Controllers/bp-camera-pawn.bp-camera-pawn_C|GetCamera _camera_pawn_reference))
  (bind _springarm (Variables|/Game/Blueprints/Controllers/bp-camera-pawn.bp-camera-pawn_C|GetSpringArm _camera_pawn_reference))
  (bind _output_get (Variables|/Script/Engine.SpringArmComponent|SetTargetArmLength _springarm (+ (Variables|/Script/Engine.SpringArmComponent|GetTargetArmLength _springarm) zoom-speed)))
  (Variables|Default|Setprevious_zoom _output_get)
  (Class|CameraComponent|SetOrthoWidth _camera (+ (Variables|/Script/Engine.CameraComponent|GetOrthoWidth _camera) zoom-speed)))