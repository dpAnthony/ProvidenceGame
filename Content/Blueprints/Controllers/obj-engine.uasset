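; Engine actor that starts the hex board game and provides keyboard and mouse hooks, largely debug in nature.
; Construction caches the board and noise renderer; BeginPlay enables input and builds the board.
; Keys rebuild the board, toggle its constant-pathing flag, or draw noise, including a per-pixel simplex grid.
; Right-click traces under the cursor to add settlement followers or print a hex's neighbor types; food/favor spawning and hex-lookup tests are disconnected.
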(event EventBeginPlay
  (bind _returnvalue (Game|GetPlayerController 0))
  (Input|SetInputModeGameandUI _returnvalue 0 "DoNotLock" false)
  (Input|EnableInput _returnvalue)
  (Default|Make-board (Variables|Default|Getboard-ref)))

(event Input|KeyboardEvents|G
  (params (Key :type Key%20Structure))
  (bind _board_ref (Variables|Default|Getboard-ref))
  (:Released
    (Variables|/Game/Blueprints/BoardGeneration/bp-board.bp-board_C|Setboard-const-pathing _board_ref (not (Variables|/Game/Blueprints/BoardGeneration/bp-board.bp-board_C|Getboard-const-pathing _board_ref)))))

(event Input|KeyboardEvents|B
  (params (Key :type Key%20Structure))
  (bind _board_ref (Variables|Default|Getboard-ref))
  (:Released
    (if (not (Variables|/Game/Blueprints/BoardGeneration/bp-board.bp-board_C|Getboard-generating (Variables|Default|Getboard-ref)))
      (bind _outactors (Actor|GetAllActorsOfClass "/Game/Objects/obj-hex.obj-hex_C"))
      (for _array_element _outactors
        (Actor|DestroyActor _array_element))
      (Utilities|Array|Clear (Variables|/Game/Blueprints/BoardGeneration/bp-board.bp-board_C|Getboard-ids (Variables|Default|Getboard-ref)))
      (Utilities|Array|Clear (Variables|/Game/Blueprints/BoardGeneration/bp-board.bp-board_C|Getboard-ids-2d (Variables|Default|Getboard-ref)))
      (Variables|/Game/Blueprints/BoardGeneration/bp-board.bp-board_C|Setboard-cur-x _board_ref 0)
      (Variables|/Game/Blueprints/BoardGeneration/bp-board.bp-board_C|Setboard-cur-y _board_ref 0)
      (Variables|/Game/Blueprints/BoardGeneration/bp-board.bp-board_C|Setboard-size _board_ref 1)
      (Default|Make-board (Variables|Default|Getboard-ref)))))

(event Input|KeyboardEvents|SpaceBar
  (params (Key :type Key%20Structure))
  (:Released
    (Default|Begin-draw (Variables|Default|Getrender-ref))
    (for _index (range 0 63)
      (for _index_2 (range 0 63)
        (bind _returnvalue (Class|SimplexNoiseBPLibrary|SimplexNoiseinRange2D (Math|Conversions|ToFloat(Integer) _index) (Math|Conversions|ToFloat(Integer) _index_2) 0.001 1.0))
        (Development|PrintString (Utilities|String|ToString(Float) _returnvalue))
        (Default|Draw-pixel (Variables|Default|Getrender-ref) _index _index_2 _returnvalue)))
    (Default|End-draw (Variables|Default|Getrender-ref))))

(event Input|KeyboardEvents|N
  (params (Key :type Key%20Structure))
  (:Released
    (Default|Make-noise-2 (Variables|Default|Getrender-ref))))

(event Input|MouseEvents|RightMouseButton
  (params (Key :type Key%20Structure))
  (:Released
    (bind _output_get (Variables|Default|Settemp-selected (.hitactor (.HitResult (Class|PlayerController|GetHitResultUnderCursorforObjects (Game|GetPlayerController 0) (Utilities|Array|MakeArray "ObjectTypeQuery1") true)))))
    (bind _asobj_settlement (Utilities|Casting|CastToobj-settlement _output_get)
      (:then
        (Default|Followers-add _asobj_settlement 10)
        (Development|PrintString (Utilities|String|ToString(Integer) (Variables|/Game/Objects/obj-settlement.obj-settlement_C|Getfollowers _asobj_settlement)))
        (if true
          _))
      (:CastFailed
        (bind _asobj_hex (Utilities|Casting|CastToobj-hex (Variables|Default|Gettemp-selected)))
        (for _array_element (Variables|/Game/Objects/obj-hex.obj-hex_C|Getneighbor-hexes _asobj_hex)
          (Development|PrintString (Variables|/Game/Objects/obj-hex.obj-hex_C|Gethex-type _array_element)))))))

(fn ConstructionScript
  (bind _outactors (Actor|GetAllActorsOfClass "/Game/Blueprints/BoardGeneration/bp-board.bp-board_C"))
  (Variables|Default|Setboard-ref (Utilities|Array|Get(acopy) _outactors))
  (bind _outactors_2 (Actor|GetAllActorsOfClass "/Game/Blueprints/BoardGeneration/bp-render-noise.bp-render-noise_C"))
  (Variables|Default|Setrender-ref (Utilities|Array|Get(acopy) _outactors_2)))