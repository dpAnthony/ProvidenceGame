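; Board-generation Blueprint that renders a 2D simplex noise texture into a render target.
; BeginPlay clears the target to black, and a separate make-noise event loops over a square grid, sampling scaled simplex noise at each coordinate.
; Each sample is drawn through the render target's canvas as a one-pixel tinted texture, offset by one pixel, between begin and end draw helper events.
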(event Custom|draw-pixel
  (params (x :type Integer) (y :type Integer) (color-float :type Float%20%28single-precision%29))
  (Variables|Default|Setdraw-x x)
  (Variables|Default|Setdraw-y y)
  (Variables|Default|Setdraw-color-float color-float)
  (Canvas|DrawTexture :self (Variables|Default|Getcanvas) :ScreenPosition (Math|Vector2D|MakeVector2D (Math|Conversions|ToFloat(Integer) (Variables|Default|Getdraw-x)) (Math|Conversions|ToFloat(Integer) (Variables|Default|Getdraw-y))) :ScreenSize "(X=1.000000,Y=1.000000)" :RenderColor (Math|Conversions|ToLinearColor(Float) (Variables|Default|Getdraw-color-float))))

(event Custom|end-draw
  (Rendering|EndDrawCanvastoRenderTarget (Variables|Default|Getcontext))
  (Variables|Default|Setdraw-x 0)
  (Variables|Default|Setdraw-y 0))

(event Custom|begin-draw
  (bind (_canvas _size _context) (Rendering|BeginDrawCanvastoRenderTarget "/Game/Materials/Textures/noise-ct.noise-ct"))
  (Variables|Default|Setcanvas _canvas)
  (Variables|Default|Setcontext _context))

(event Custom|make-noise-2
  (bind _noise_scale (Variables|Default|Getnoise-scale))
  (CallFunction|Begin-draw)
  (for _index (range 0 (Variables|Default|Getwidth))
    (Variables|Default|Setdraw-y _index)
    (for _index_2 (range 0 (Variables|Default|Getwidth))
      (Variables|Default|Setdraw-x _index_2)
      (bind _returnvalue (Class|SimplexNoiseBPLibrary|SimplexNoiseinRange2D (* (Math|Conversions|ToFloat(Integer) (Variables|Default|Getdraw-x)) _noise_scale) (* (Math|Conversions|ToFloat(Integer) (Variables|Default|Getdraw-y)) _noise_scale) 0.0 1.0))
      (CallFunction|Draw-pixel (+ (Variables|Default|Getdraw-x) 1) (+ (Variables|Default|Getdraw-y) 1) (Math|Float|Absolute(Float) _returnvalue))))
  (CallFunction|End-draw))

(event EventBeginPlay
  (Rendering|ClearRenderTarget2D "/Game/Materials/Textures/noise-ct.noise-ct"))

(fn ConstructionScript)