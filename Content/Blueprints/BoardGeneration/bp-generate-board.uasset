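; Board generation Blueprint that, as it stands, only provides a lookup from board coordinates to a flat index.
; The index function accepts a coordinate type with axial, array and cube inputs, and computes array Y times board height plus array X.
; The cube case shares that array formula without converting its inputs, and no axial case is handled.
; The construction script is empty, so no board is built here.
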(fn ConstructionScript)

(fn Board-get-index
  (params (coordinate-type :type String) (axial-x :type Integer) (axial-y :type Integer) (array-x :type Integer) (array-y :type Integer) (cube-x :type Integer) (cube-y :type Integer) (cube-z :type Integer))
  (LocalVariables|Setlocal-coordinate-type coordinate-type)
  (LocalVariables|Setlocal-axial-x axial-x)
  (LocalVariables|Setlocal-axial-y axial-y)
  (LocalVariables|Setlocal-array-x array-x)
  (LocalVariables|Setlocal-array-y array-y)
  (LocalVariables|Setlocal-cube-x cube-x)
  (LocalVariables|Setlocal-cube-y cube-y)
  (LocalVariables|Setlocal-cube-z cube-z)
  (switch string (LocalVariables|Getlocal-coordinate-type)
    (:array
      _)
    (:cube
      _))
  (return (+ (* (LocalVariables|Getlocal-array-y) (LocalVariables|Getboard-height)) (LocalVariables|Getlocal-array-x))))